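; Player shield Blueprint that takes damage when enemies overlap its sphere and sounds an alarm when it goes down.
; BP_AirburstEnemy and MediumEnemy_BP overlaps call ShieldTakeDamage with their respective damage values.
; Airburst hits also create a dynamic material, set the impact position and animate a ripple radius through a timeline.
; Tick uses a DoOnce to play the alarm once while inactive, re-arming whenever shield health is above zero.
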(event OnComponentBeginOverlap(Sphere)
  (params (OverlappedComponent :type Primitive%20Component%20Object%20Reference) (OtherActor :type Actor%20Object%20Reference) (OtherComp :type Primitive%20Component%20Object%20Reference) (OtherBodyIndex :type Integer) (bFromSweep :type Boolean) (SweepResult :type Hit%20Result%20Structure%20%28by%20ref%29))
  (Utilities|FlowControl|Sequence
    (:then_0
      (Utilities|Casting|CastToBP_AirburstEnemy OtherActor)
      (Class|Sheild|ShieldTakeDamage (Variables|Default|GetProjectile%20Damage))
      (bind _returnvalue (Rendering|Material|CreateDynamicMaterialInstance (Variables|Default|GetSphere) 0 0 "None" :!class /Script/Engine.PrimitiveComponent))
      (Rendering|Material|SetVectorParameterValue _returnvalue "Pos" (Math|Conversions|ToLinearColor(Vector) (.impactpoint SweepResult)) :!class /Script/Engine.MaterialInstanceDynamic)
      (bind _新建轨迹_0 (Timeline|时间轴_0 PlayFromStart)
        (:Update
          (Rendering|Material|SetScalarParameterValue _returnvalue "Radius" (* _新建轨迹_0 2e+03) :!class /Script/Engine.MaterialInstanceDynamic))))
    (:then_1
      (Utilities|Casting|CastToMediumEnemy_BP OtherActor)
      (Class|Sheild|ShieldTakeDamage (Variables|Default|GetMedium%20Enemy%20Damage)))))

(event EventTick
  (params (DeltaSeconds :type Float%20%28single-precision%29))
  (Utilities|FlowControl|Sequence
    (:then_0
      (if (not (Variables|Default|GetIsShieldActive))
        (Utilities|FlowControl|DoOnce false :!label _label
          (:Completed
            (Audio|PlaySoundatLocation "/Game/Cosco/Audio/Shields_Down_Alarm.Shields_Down_Alarm" "0, 0, 0" "0, 0, 0" 1.0 1.0 0.0 0 0 0)))))
    (:then_1
      (if (> (Variables|Default|GetShieldHealth) 0.0)
        (goto _label Reset)))))

(fn ConstructionScript)