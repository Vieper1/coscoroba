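; Dummy player character for multiplayer that relays each player's input to the shared HMC_Coscoroba actor, found in the construction script.
; ControllerSettings decides which camera axis the player feeds to Coscoroba and whether Fire triggers Airburst or Gatling.
; Menu navigation inputs record the player as index 0 or 1 in PlayerSettings, then call UI navigation events.
; Authority-based online/local weapon-control logic remains as disconnected, mostly empty stubs.
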(event Custom|MoveRightOnser
  (params (Right :type Float%20%28single-precision%29))
  ;[1 1 1] Run OnServer events
  ;;[1 1 1] Move Right On Server
)

(event Collision|EventActorBeginOverlap
  (params (OtherActor :type Actor%20Object%20Reference)))

(event EventTick
  (params (DeltaSeconds :type Float%20%28single-precision%29)))

(event Input|ActionEvents|InputActionUI_nav_down
  (params (Key :type Key%20Structure :default "None"))
  ;[1 1 1] For StartMenu
  (:Pressed
    (CallFunction|SetCurrentPlayer)
    (Default|CallUINavDownEvent)))

(event Input|ActionEvents|InputActionUI_nav_up
  (params (Key :type Key%20Structure :default "None"))
  ;[1 1 1] For StartMenu
  (:Pressed
    (CallFunction|SetCurrentPlayer)
    (Default|CallUINavUpEvent)))

(event Input|ActionEvents|InputActionUI_nav_left
  (params (Key :type Key%20Structure :default "None"))
  ;[1 1 1] For StartMenu
  (:Pressed
    (CallFunction|SetCurrentPlayer)
    (Default|CallUINavLeftEvent)))

(event Input|ActionEvents|InputActionUI_nav_right
  (params (Key :type Key%20Structure :default "None"))
  ;[1 1 1] For StartMenu
  (:Pressed
    (CallFunction|SetCurrentPlayer)
    (Default|CallUINavRightEvent)))

(event Input|ActionEvents|InputActionFire
  (params (Key :type Key%20Structure :default "None"))
  (bind _controllersettings (Variables|Default|GetControllerSettings))
  (bind _coscorobaref (Variables|Default|GetCoscorobaRef))
  ;[1 1 1] With One Dummy Char & Coscoroba himself
  ;;[1 1 1] Fire Weapon
  (:Pressed
    (Utilities|IsValid (Variables|Default|GetCoscorobaRef)
      (:Is%20Valid
        (switch Utilities|FlowControl|Switch|SwitchonEFireControl (.firesettings _controllersettings)
          (:Airburst
            (Default|FireAirburst _coscorobaref true))
          (:Gatling
            (Default|FireGatling _coscorobaref true))))))
  (:Released
    (Utilities|IsValid (Variables|Default|GetCoscorobaRef)
      (:Is%20Valid
        (switch Utilities|FlowControl|Switch|SwitchonEFireControl (.firesettings _controllersettings)
          (:Airburst
            (Default|FireAirburst _coscorobaref false))
          (:Gatling
            (Default|FireGatling _coscorobaref false)))))))

(event Input|AxisEvents|InputAxisTurnRate
  (params (AxisValue :type Float%20%28single-precision%29))
  (bind _controllersettings (Variables|Default|GetControllerSettings))
  (bind _coscorobaref (Variables|Default|GetCoscorobaRef))
  ;[1 1 1] With One Dummy Char & Coscoroba himself
  ;;[1 1 1] Camera Movement
  (Utilities|IsValid (Variables|Default|GetCoscorobaRef)
    (:Is%20Valid
      (switch Utilities|FlowControl|Switch|SwitchonECameraControl (.cameracontrolsettings _controllersettings)
        (:TurnRight
          (Class|CoscoCameraCharacter|TakeInputforLocalMulPlayer _coscorobaref (.cameracontrolsettings _controllersettings) AxisValue))
        (:LookUp
          (Class|CoscoCameraCharacter|TakeInputforLocalMulPlayer _coscorobaref (.cameracontrolsettings _controllersettings) (stale Input|AxisEvents|InputAxisLookUpRate AxisValue)))))))

(event Input|AxisEvents|InputAxisLookUpRate
  (params (AxisValue :type Float%20%28single-precision%29))
  (bind _controllersettings (Variables|Default|GetControllerSettings))
  (bind _coscorobaref (Variables|Default|GetCoscorobaRef))
  ;[1 1 1] With One Dummy Char & Coscoroba himself
  ;;[1 1 1] Camera Movement
  (Utilities|IsValid (Variables|Default|GetCoscorobaRef)
    (:Is%20Valid
      (switch Utilities|FlowControl|Switch|SwitchonECameraControl (.cameracontrolsettings _controllersettings)
        (:TurnRight
          (Class|CoscoCameraCharacter|TakeInputforLocalMulPlayer _coscorobaref (.cameracontrolsettings _controllersettings) (stale Input|AxisEvents|InputAxisTurnRate AxisValue)))
        (:LookUp
          (Class|CoscoCameraCharacter|TakeInputforLocalMulPlayer _coscorobaref (.cameracontrolsettings _controllersettings) AxisValue))))))

(fn ConstructionScript
  (bind _returnvalue (Actor|GetActorOfClass "/Game/Cosco/Blueprints/XShip/HMC_Coscoroba.HMC_Coscoroba_C"))
  (Variables|Default|SetCoscorobaRef _returnvalue))

(fn ControlWeapons
  (params (IsOnline :type Boolean) (AxisValue :type Float%20%28single-precision%29) (IsLookUp :type Boolean))
  (if IsOnline
    (CallFunction|Online AxisValue IsLookUp)
    (else
      (CallFunction|Local AxisValue IsLookUp))))

(fn Online
  (params (Axis%20Value :type Float%20%28single-precision%29) (IsLookUp :type Boolean))
  (bind _coscorobaref (Variables|Default|GetCoscorobaRef))
  (if IsLookUp
    (Networking|SwitchHasAuthority
      (:Authority
        (Utilities|IsValid _coscorobaref)))
    (else
      (Networking|SwitchHasAuthority
        (:Remote
          (Utilities|IsValid _coscorobaref
            (:Is%20Valid
              (CallFunction|MOveRightOnser Axis%20Value))))))))

(fn Local
  (params (Axis%20Value :type Float%20%28single-precision%29) (IsLookUp :type Boolean))
  (if (not IsLookUp)
    (if (== (Pawn|GetControlledPawn (Game|GetPlayerController 1)) self)
      (Utilities|IsValid (Variables|Default|GetCoscorobaRef)))))

(fn SetCurrentPlayer
  (if (== self (Pawn|GetControlledPawn (Game|GetPlayerController 0)))
    (bind _asplayer_settings (Utilities|Casting|CastToPlayerSettings (Game|GetGameInstance)))
    (Variables|/Game/Cosco/PlayerSettings.PlayerSettings_C|SetCurrentPlayerIndex _asplayer_settings 0)
    (else
      (bind _asplayer_settings_2 (Utilities|Casting|CastToPlayerSettings (Game|GetGameInstance)))
      (Variables|/Game/Cosco/PlayerSettings.PlayerSettings_C|SetCurrentPlayerIndex _asplayer_settings_2 1))))