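; BP_Airburst is an airburst projectile that handles its firing and explosion sounds and carries its shooter's velocity.
; On BeginPlay, outside SplashLevel, it plays a muzzle sound and binds OnDestroyed to an attenuated explosion sound.
; It also caches the instigator's FakeVelocity, which Tick applies as an unswept world offset using a fixed time step rather than delta time.
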(event Custom|OnDestroy
  (params (DestroyedActor :type Actor%20Object%20Reference))
  (Audio|PlaySoundatLocation "/Game/Bofor/Sounds/Raw/2/Explosion_2.Explosion_2" (Transformation|GetActorLocation DestroyedActor) "0, 0, 0" 1.0 1.0 0.0 "/Game/Cosco/Audio/GeneralAttenuation.GeneralAttenuation" 0 0))

(event EventTick
  (params (DeltaSeconds :type Float%20%28single-precision%29))
  (Transformation|AddActorWorldOffset (* (Variables|Default|GetSpawnerVelocity) 0.015)))

(event EventBeginPlay
  (Utilities|FlowControl|Sequence
    (:then_0
      (bind _returnvalue (Game|GetCurrentLevelName true))
      (if (not (Utilities|Enum|Equal(Enum) _returnvalue "SplashLevel"))
        (Audio|PlaySoundatLocation (Variables|Default|GetMuzzleSound) (Transformation|GetActorLocation) "0, 0, 0" 1.0 1.0 0.0 0 0 0)
        (Game|BindEventtoOnDestroyed (delegate Custom|OnDestroy))))
    (:then_1
      (Variables|Default|SetSpawnerVelocity (Variables|/Script/Bofor.CoscoBaseCharacter|GetFakeVelocity (Variables|Default|GetInstigatorActor))))))

(fn ConstructionScript)