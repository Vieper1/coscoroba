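; Player ship Blueprint, Coscoroba2, that switches between Airburst and Gatling turrets when not firing and displays enemy radars.
; BeginPlay feeds actors of two enemy classes into a 3D widget radar and a delayed viewport radar.
; A left/right radar, rebuilt on a timer with camera-relative yaw and pitch filters, exists but its setup never runs.
; Tick prints camera rotation for debugging, and interface getters expose mesh location and camera rotation.
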(event Custom|HandleRadar
  (Utilities|Time|SetTimerbyFunctionName 0 "HandleRadarTargets" 1.0 true))

(event Custom|Setup3DRadar
  (bind _3dradarwidget (Variables|Default|Get3DradarWidget))
  (Development|SetHiddeninGame _3dradarwidget false false)
  (bind _as3dradar_widget (Utilities|Casting|CastTo3DradarWidget (UserInterface|GetUserWidgetObject _3dradarwidget)))
  (bind _output_get (Variables|Default|Set3DRadarComponent (Variables|/Game/UMGRadar/2-CarExample/Widgets/3DradarWidget.3DradarWidget_C|GetUMGRadarWidgetComponent _as3dradar_widget)))
  (Default|RadarUpdate _output_get self)
  (CallFunction|AddEnemiesforRadar "/Game/Spline/Plane_Damageable1.Plane_Damageable1_C" (Variables|/Game/UMGRadar/2-CarExample/Widgets/3DradarWidget.3DradarWidget_C|GetUMGRadarWidgetComponent _as3dradar_widget) "/Game/UMGRadar/Images/R_playerLoc.R_playerLoc" "(X=50.000000,Y=50.000000)" "(R=0.833333,G=0.210991,B=0.831867,A=1.000000)" false)
  (CallFunction|AddEnemiesforRadar "/Game/Cosco/Blueprints/Enemy/LightEnemyForRadar.LightEnemyForRadar_C" (Variables|/Game/UMGRadar/2-CarExample/Widgets/3DradarWidget.3DradarWidget_C|GetUMGRadarWidgetComponent _as3dradar_widget) "/Game/UMGRadar/Images/Light_Enemy.Light_Enemy" "(X=50.000000,Y=50.000000)" "(R=0.240258,G=0.833333,B=0.049916,A=1.000000)" false))

(event EventBeginPlay
  (|CallParentFunction)
  (CallFunction|Setup3DRadar)
  (bind _returnvalue (UserInterface|CreateWidget "/Game/UMGRadar/UMGRadar.UMGRadar_C"))
  (bind _output_get (Variables|Default|SetRadarHMC2 _returnvalue))
  (Utilities|FlowControl|Delay 2.0)
  (UserInterface|Viewport|AddtoViewport _returnvalue 0)
  (Default|RadarUpdate (Variables|/Game/UMGRadar/UMGRadar.UMGRadar_C|GetUMGRadarWidgetComponent _output_get) self)
  (CallFunction|AddEnemiesforRadar "/Game/Spline/Plane_Damageable1.Plane_Damageable1_C" (Variables|/Game/UMGRadar/UMGRadar.UMGRadar_C|GetUMGRadarWidgetComponent (Variables|Default|GetRadarHMC2)) "/Game/UMGRadar/Images/R_playerLoc.R_playerLoc" "(X=50.000000,Y=50.000000)" "(R=0.833333,G=0.210991,B=0.831867,A=1.000000)" false)
  (CallFunction|AddEnemiesforRadar "/Game/Cosco/Blueprints/Enemy/LightEnemyForRadar.LightEnemyForRadar_C" (Variables|/Game/UMGRadar/UMGRadar.UMGRadar_C|GetUMGRadarWidgetComponent (Variables|Default|GetRadarHMC2)) "/Game/UMGRadar/Images/Light_Enemy.Light_Enemy" "(X=50.000000,Y=50.000000)" "(R=0.240258,G=0.833333,B=0.049916,A=1.000000)" false))

(event EventTick
  (params (DeltaSeconds :type Float%20%28single-precision%29))
  (|CallParentFunction DeltaSeconds)
  (Development|PrintString (Utilities|String|ToString(Rotator) (Transformation|GetWorldRotation (Variables|Default|GetMainCamera))) true true "(R=0.000000,G=0.660000,B=1.000000,A=1.000000)" 0.0))

(event Input|ActionEvents|InputActionFire
  (params (Key :type Key%20Structure :default "None"))
  (:Released
    (if (Utilities|Enum|Equal(Enum) (Variables|Default|GetCurrentWeaponMode) "WS_Gatling")
      (Variables|Default|SetbIsFiring false))))

(event Input|KeyboardEvents|1
  (params (Key :type Key%20Structure :default "None"))
  ;[1 1 1] Switch to Airburst
  (:Pressed
    (if (and (Utilities|Enum|NotEqual(Enum) (Variables|Default|GetCurrentWeaponMode) "WS_Airburst") (not (Variables|Default|GetbIsFiring)))
      (Variables|Default|SetCurrentWeaponMode "WS_Airburst")
      (Utilities|Struct|SetmembersinTurret (Utilities|Array|Get(acopy) (Variables|Default|GetProjectiles)) true)
      (Utilities|Struct|SetmembersinTurret (Utilities|Array|Get(acopy) (Variables|Default|GetProjectiles) 1) false))))

(event Input|KeyboardEvents|2
  (params (Key :type Key%20Structure :default "None"))
  ;[1 1 1] Switch to Gatling
  (:Pressed
    (if (and (Utilities|Enum|NotEqual(Enum) (Variables|Default|GetCurrentWeaponMode) "WS_Gatling") (not (Variables|Default|GetbIsFiring)))
      (Variables|Default|SetCurrentWeaponMode "WS_Gatling")
      (Utilities|Struct|SetmembersinTurret (Utilities|Array|Get(acopy) (Variables|Default|GetProjectiles)) false)
      (Utilities|Struct|SetmembersinTurret (Utilities|Array|Get(acopy) (Variables|Default|GetProjectiles) 1) true))))

(fn ConstructionScript)

(fn AddEnemiesforRadar
  (params (ActorClass :type Actor%20Class%20Reference) (Target :type UMG%20Radar%20Widget%20Component%20Object%20Reference) (Texture :type Texture%202D%20Object%20Reference) (OffScreenTextureSize :type Vector%202D%20Structure) (Specified%20Color :type Linear%20Color%20Structure) (bIsPersistent :type Boolean))
  (bind _outactors (Actor|GetAllActorsOfClass ActorClass))
  (Default|AddTargetActors Target _outactors bIsPersistent true Texture "(X=50.000000,Y=50.000000)" (Utilities|Struct|MakeSlateColor Specified%20Color) false "" "/Game/UMGRadar/Images/R_OffScreenArrow.R_OffScreenArrow" OffScreenTextureSize false 1.0))

(fn AddTargets
  (params (ActorClassType :type Actor%20Class%20Reference) (EnemyTexture :type Texture%202D%20Object%20Reference) (FollowRotation :type Boolean) (Specified%20Color :type Linear%20Color%20Structure))
  (bind _radarleftright (Variables|Default|GetRadarLeftRight))
  (bind _outactors (Actor|GetAllActorsOfClass ActorClassType))
  (bind _locationvector (CallFunction|ITGetLocation))
  (bind _rotation (CallFunction|ITGetRotation))
  (for _array_element _outactors
    (bind _locationvector_2 (Class|RadarRotationInterface|ITGetLocation(Message) _array_element))
    (if (Math|Float|InRange(Float) (.yaw (Math|Rotator|Delta(Rotator) (Math|Rotator|FindLookatRotation _locationvector _locationvector_2) _rotation)) -9e+01 9e+01)
      (bind _output_get (Variables|Default|SetDiff%20Yaw (.pitch (Math|Rotator|Delta(Rotator) (Math|Rotator|FindLookatRotation _locationvector _locationvector_2) _rotation))))
      (Utilities|FlowControl|Sequence
        (:then_0
          (Default|AddTargetActor (Variables|/Game/UMGRadar/UMGRadar2.UMGRadar2_C|GetRadarLeft _radarleftright) _array_element false FollowRotation EnemyTexture "(X=50.000000,Y=50.000000)" (Utilities|Struct|MakeSlateColor Specified%20Color) false "" 0 "(X=50.000000,Y=50.000000)" false 1.0))
        (:then_1
          (if (Math|Float|InRange(Float) _output_get -25.0 25.0)
            (Default|AddTargetActor (Variables|/Game/UMGRadar/UMGRadar2.UMGRadar2_C|GetRadarRight _radarleftright) _array_element false FollowRotation EnemyTexture "(X=50.000000,Y=50.000000)" (Utilities|Struct|MakeSlateColor Specified%20Color) false "" 0 "(X=50.000000,Y=50.000000)" false 1.0)))))))

(fn HandleRadarTargets
  (Default|RemoveAllTargets (Variables|/Game/UMGRadar/UMGRadar2.UMGRadar2_C|GetRadarLeft (Variables|Default|GetRadarLeftRight)))
  (CallFunction|AddTargets "/Game/Spline/Plane_Damageable1.Plane_Damageable1_C" "/Game/UMGRadar/Images/R_playerLoc.R_playerLoc" true "(R=0.000000,G=0.000000,B=0.000000,A=1.000000)")
  (CallFunction|AddTargets "/Game/Spline/Plane_Damageable.Plane_Damageable_C" "/Game/UMGRadar/Images/R_playerLoc.R_playerLoc" true "(R=0.520833,G=0.099921,B=0.073242,A=1.000000)"))

(fn ITGetLocation
  (return (Transformation|GetWorldLocation (Variables|Default|GetMainMesh))))

(fn ITGetRotation
  (return (Transformation|GetWorldRotation (Variables|Default|GetMainCamera))))