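; HMC_GameMode is a game mode that provides enemy-hit feedback and voiceover playback.
; IndicateDamageEnemy casts the first player pawn to HMC_Coscoroba and, if its crosshair widget is valid, triggers DamageDealtCross.
; PlayVoiceLine selects the Bridge, Captain, Crewman or Navigator sound component by voice type, sets its integer ID parameter to choose the line, then plays it.
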(fn ConstructionScript)

(fn IndicateDamageEnemy
  (bind _ashmc_coscoroba (Utilities|Casting|CastToHMC_Coscoroba (Game|Player|GetPlayerPawn 0)))
  (Utilities|IsValid (Variables|/Game/Cosco/Blueprints/XShip/HMC_Coscoroba.HMC_Coscoroba_C|GetWidget_Crosshair _ashmc_coscoroba)
    (:Is%20Valid
      (Default|DamageDealtCross (Variables|/Game/Cosco/Blueprints/XShip/HMC_Coscoroba.HMC_Coscoroba_C|GetWidget_Crosshair _ashmc_coscoroba)))))

(fn PlayVoiceLine
  (params (VoiceType :type VoiceType%20Enum :default "NewEnumerator0") (ID :type Integer))
  (bind _sound_voiceover_navigator (Variables|Voice|GetSound_Voiceover_Navigator))
  (bind _sound_voiceover_bridge (Variables|Voice|GetSound_Voiceover_Bridge))
  (bind _sound_voiceover_captain (Variables|Voice|GetSound_Voiceover_Captain))
  (bind _sound_voiceover_crewman (Variables|Voice|GetSound_Voiceover_Crewman))
  (switch Utilities|FlowControl|Switch|SwitchonVoiceType VoiceType
    (:NewEnumerator0
      (Components|Activation|Activate _sound_voiceover_bridge false)
      (Effects|Components|ParticleSystem|SetIntParameter _sound_voiceover_bridge "ID" ID)
      (Audio|Components|Audio|Play _sound_voiceover_bridge 0.0))
    (:NewEnumerator1
      (Components|Activation|Activate _sound_voiceover_captain false)
      (Effects|Components|ParticleSystem|SetIntParameter _sound_voiceover_captain "ID" ID)
      (Audio|Components|Audio|Play _sound_voiceover_captain 0.0))
    (:NewEnumerator2
      (Components|Activation|Activate _sound_voiceover_crewman false)
      (Effects|Components|ParticleSystem|SetIntParameter _sound_voiceover_crewman "ID" ID)
      (Audio|Components|Audio|Play _sound_voiceover_crewman 0.0))
    (:NewEnumerator3
      (Components|Activation|Activate _sound_voiceover_navigator false)
      (Effects|Components|ParticleSystem|SetIntParameter _sound_voiceover_navigator "ID" ID)
      (Audio|Components|Audio|Play _sound_voiceover_navigator 0.0))))