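; Test player ship Blueprint with two switchable weapons, Airburst and Gatling, plus a shield and cockpit dashboard.
; Keys 1 and 2 switch modes when not firing, toggling turret projectile entries, switch audio and crosshair widget.
; BeginPlay spawns the optional shield and crosshair; Tick feeds shield health and state into health bar and warning bulb material parameters.
; Helper functions jitter mesh rotation and destroy heat-sink bulbs one at a time.
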(event EventTick
  (params (DeltaSeconds :type Float%20%28single-precision%29))
  (Utilities|FlowControl|Sequence
    (:then_0
      (Utilities|TickDashboardUpdate))))

(event EventBeginPlay
  (Utilities|FlowControl|Sequence
    (:then_0
      (Utilities|InitShield))
    (:then_1
      (Utilities|InitCrosshairWidget))))

(event Input|ActionEvents|InputActionFire
  (params (Key :type Key%20Structure :default "None"))
  (:Released
    (if (Utilities|Enum|Equal(Enum) (Variables|Default|GetCurrentWeaponMode) "WS_Gatling")
      (Variables|Default|SetbIsFiring false))))

(event Input|KeyboardEvents|1
  (params (Key :type Key%20Structure :default "None"))
  ;[1 1 1] Switch to Airburst
  (:Pressed
    (if (and (Utilities|Enum|NotEqual(Enum) (Variables|Default|GetCurrentWeaponMode) "WS_Airburst") (not (Variables|Default|GetbIsFiring)))
      (Variables|Default|SetCurrentWeaponMode "WS_Airburst")
      (Utilities|Struct|SetmembersinTurret (Utilities|Array|Get(acopy) (Variables|Default|GetProjectiles)) true)
      (Utilities|Struct|SetmembersinTurret (Utilities|Array|Get(acopy) (Variables|Default|GetProjectiles) 1) false)
      (CallFunction|SoundSwitchWeapon (Variables|Default|GetCurrentWeaponMode))
      (Default|WeaponSwitchAirburst (Variables|Default|GetWidget_Crosshair)))))

(event Input|KeyboardEvents|2
  (params (Key :type Key%20Structure :default "None"))
  ;[1 1 1] Switch to Gatling
  (:Pressed
    (if (and (Utilities|Enum|NotEqual(Enum) (Variables|Default|GetCurrentWeaponMode) "WS_Gatling") (not (Variables|Default|GetbIsFiring)))
      (Variables|Default|SetCurrentWeaponMode "WS_Gatling")
      (Utilities|Struct|SetmembersinTurret (Utilities|Array|Get(acopy) (Variables|Default|GetProjectiles)) false)
      (Utilities|Struct|SetmembersinTurret (Utilities|Array|Get(acopy) (Variables|Default|GetProjectiles) 1) true)
      (CallFunction|SoundSwitchWeapon (Variables|Default|GetCurrentWeaponMode))
      (Default|WeaponSwitchGatling (Variables|Default|GetWidget_Crosshair)))))

(fn ConstructionScript)

(fn SoundSwitchWeapon
  (params (WeaponMode :type EWeaponMode%20Enum :default "WS_Airburst"))
  (bind _sound_weaponswitcher (Variables|Default|GetSound_WeaponSwitcher))
  (Effects|Components|ParticleSystem|SetIntParameter _sound_weaponswitcher "WeaponMode" (Math|Conversions|ToInteger(Byte) WeaponMode))
  (Audio|Components|Audio|Play _sound_weaponswitcher 0.0))

(fn Shaking
  (Transformation|SetWorldRotation (Variables|Default|GetMainMesh) (Math|Rotator|MakeRotator (+ (Variables|CloudLevelRotation|GetRoll) (Math|Random|RandomFloatinRange -0.5 0.5)) (+ (Variables|CloudLevelRotation|GetPitch) (Math|Random|RandomFloatinRange -0.5 0.5)) (+ (Variables|CloudLevelRotation|GetYaw) (Math|Random|RandomFloatinRange -0.5 0.5))) false false))