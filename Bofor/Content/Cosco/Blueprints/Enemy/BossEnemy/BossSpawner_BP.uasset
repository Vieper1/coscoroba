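; Boss spawner that creates a BossEnemy_BP when the HMC_Coscoroba character overlaps its Trigger component.
; The boss spawns at the first point of the referenced Spline actor and receives that spline, a movement speed and the FireTrigger actor.
; Nothing guards against repeat spawns on later overlaps.
; The spawner's own FireTrigger overlap event is empty, leaving its FireBDG call disconnected.
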(event OnComponentBeginOverlap(Trigger)
  (params (OverlappedComponent :type Primitive%20Component%20Object%20Reference) (OtherActor :type Actor%20Object%20Reference) (OtherComp :type Primitive%20Component%20Object%20Reference) (OtherBodyIndex :type Integer) (bFromSweep :type Boolean) (SweepResult :type Hit%20Result%20Structure%20%28by%20ref%29))
  (Utilities|Casting|CastToHMC_Coscoroba OtherActor)
  (bind _returnvalue (Game|SpawnActorfromClass "/Game/Cosco/Blueprints/Enemy/BossEnemy/BossEnemy_BP.BossEnemy_BP_C" (Math|Transform|MakeTransform (Spline|GetLocationatSplinePoint (Variables|/Script/Bofor.SplineActor|GetSpline (Variables|Default|GetSpline)) 0 "World") "0, 0, 0" "1,1,1") "AlwaysSpawn" 0 0 0))
  (Utilities|FlowControl|Sequence
    (:then_0
      (Variables|/Script/Bofor.CoscoBaseCharacter|SetMySplineActor _returnvalue (Variables|Default|GetSpline)))
    (:then_1
      (Variables|/Script/Bofor.CoscoBaseCharacter|Setm_Speed _returnvalue (Variables|Default|GetSpeed)))
    (:then_2
      (Variables|/Game/Cosco/Blueprints/Enemy/BossEnemy/BossEnemy_BP.BossEnemy_BP_C|SetFireTriggerBDG _returnvalue (Variables|Default|GetFireTrigger)))))

(event OnActorBeginOverlap(FireTrigger)
  (params (OverlappedActor :type Actor%20Object%20Reference) (OtherActor :type Actor%20Object%20Reference)))

(event EventBeginPlay)

(event Collision|EventActorBeginOverlap
  (params (OtherActor :type Actor%20Object%20Reference)))

(event EventTick
  (params (DeltaSeconds :type Float%20%28single-precision%29)))

(fn ConstructionScript)