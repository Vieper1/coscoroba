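; Trigger-volume spawner that creates medium enemies when the player character, HMC_Coscoroba, overlaps it.
; For each entry in its spawn struct array, it spawns a MediumEnemy_BP at the first point of that entry's spline actor.
; It then copies the spline, damage, range, dash and speed settings onto the enemy, and uses the lerp time as the play rate of its speed ramp timelines.
; Nothing disables the trigger, so every qualifying overlap spawns a new set.
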(event OnComponentBeginOverlap(Trigger)
  (params (OverlappedComponent :type Primitive%20Component%20Object%20Reference) (OtherActor :type Actor%20Object%20Reference) (OtherComp :type Primitive%20Component%20Object%20Reference) (OtherBodyIndex :type Integer) (bFromSweep :type Boolean) (SweepResult :type Hit%20Result%20Structure%20%28by%20ref%29))
  (Utilities|Casting|CastToHMC_Coscoroba OtherActor)
  (for _array_element (Variables|Default|GetMD_SpawnStructs)
    (bind _returnvalue (Game|SpawnActorfromClass "/Game/Cosco/Blueprints/Enemy/Medium/MediumEnemy_BP.MediumEnemy_BP_C" (Math|Transform|MakeTransform (Spline|GetLocationatSplinePoint (Variables|/Script/Bofor.SplineActor|GetSpline (.SplineActor (Utilities|Struct|BreakMDSpawn_Struct _array_element))) 0 "World") "0, 0, 0" "1,1,1") "AlwaysSpawn" 0 0))
    (Utilities|FlowControl|Sequence
      (:then_0
        (Variables|/Script/Bofor.CoscoBaseCharacter|SetMySplineActor _returnvalue (.SplineActor (Utilities|Struct|BreakMDSpawn_Struct _array_element))))
      (:then_1
        (Variables|/Game/Cosco/Blueprints/Enemy/Medium/MediumEnemy_BP.MediumEnemy_BP_C|SetAmountOfDamage _returnvalue (.AmountOfDamage (Utilities|Struct|BreakMDSpawn_Struct _array_element))))
      (:then_2
        (Variables|/Script/Bofor.CoscoEnemyCharacter|SetRange _returnvalue (.Range (Utilities|Struct|BreakMDSpawn_Struct _array_element))))
      (:then_3
        (Variables|/Game/Cosco/Blueprints/Enemy/Medium/MediumEnemy_BP.MediumEnemy_BP_C|SetDashMultiplier _returnvalue (.DashMultiplier (Utilities|Struct|BreakMDSpawn_Struct _array_element))))
      (:then_4
        (bind _output_get (Variables|/Game/Cosco/Blueprints/Enemy/Medium/MediumEnemy_BP.MediumEnemy_BP_C|SetLerpTime _returnvalue (.LerpTime (Utilities|Struct|BreakMDSpawn_Struct _array_element))))
        (Components|Timeline|SetPlayRate (Variables|/Game/Cosco/Blueprints/Enemy/Medium/MediumEnemy_BP.MediumEnemy_BP_C|GetSpeedRamup _returnvalue) _output_get)
        (Components|Timeline|SetPlayRate (Variables|/Game/Cosco/Blueprints/Enemy/Medium/MediumEnemy_BP.MediumEnemy_BP_C|GetSpeedRamDown _returnvalue) _output_get))
      (:then_5
        (bind _output_get_2 (Variables|/Script/Bofor.CoscoBaseCharacter|Setm_Speed _returnvalue (.Speed (Utilities|Struct|BreakMDSpawn_Struct _array_element))))
        (Variables|/Game/Cosco/Blueprints/Enemy/Medium/MediumEnemy_BP.MediumEnemy_BP_C|SetinitialSpeed _returnvalue _output_get_2)))))

(event EventBeginPlay)

(event Collision|EventActorBeginOverlap
  (params (OtherActor :type Actor%20Object%20Reference)))

(event EventTick
  (params (DeltaSeconds :type Float%20%28single-precision%29)))

(fn ConstructionScript)