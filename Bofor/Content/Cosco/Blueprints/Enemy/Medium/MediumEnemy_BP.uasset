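; Medium enemy that registers on the player's radar, dashes when the player is ahead, and damages them on contact before exploding.
; A forward sphere trace drives two timelines that ramp MSpeed up and back down.
; At low health it drops its spline and falls smoking under gravity, carried by velocity calculated from position deltas, exploding on non-projectile overlap.
; The charge-at-player and crash-timeline logic is unconnected.
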(event OnComponentBeginOverlap(MainMesh)
  (params (OverlappedComponent :type Primitive%20Component%20Object%20Reference) (OtherActor :type Actor%20Object%20Reference) (OtherComp :type Primitive%20Component%20Object%20Reference) (OtherBodyIndex :type Integer) (bFromSweep :type Boolean) (SweepResult :type Hit%20Result%20Structure%20%28by%20ref%29))
  ;[1 1 1] On Collision
  (if (Variables|Default|GetIsAlive)
    (bind _ashmc_coscoroba (Utilities|Casting|CastToHMC_Coscoroba OtherActor))
    (Class|CoscoBaseCharacter|TakeDamage _ashmc_coscoroba (Variables|Enemy|GetAmountOfDamage))
    (CallFunction|Explode)
    (else
      (Utilities|Casting|CastToBaseProjectile OtherActor
        (:CastFailed
          (CallFunction|Explode))))))

(event EventBeginPlay
  (bind _lerptime (Variables|Enemy|GetLerpTime))
  ;[1 1 1] Begin Play
  (Utilities|FlowControl|Delay 0.2)
  (bind _ashmc_coscoroba (Utilities|Casting|CastToHMC_Coscoroba (Game|Player|GetPlayerPawn 0)))
  (bind _output_get (Variables|Default|SetPlayerRef _ashmc_coscoroba))
  (Variables|Default|SetinitialSpeed (Variables|Default|Getm_Speed))
  (Components|Timeline|SetPlayRate (Variables|Default|GetSpeedRamup) _lerptime)
  (Components|Timeline|SetPlayRate (Variables|Default|GetSpeedRamDown) _lerptime)
  (Default|PleaseAddmetoRadar _output_get self "(R=0.385417,G=0.698077,B=1.000000,A=1.000000)" "(X=30.000000,Y=30.000000)"))

(event EventOnTakeDamage
  ;[1 1 1] On Collision
  (Utilities|FlowControl|Sequence
    (:then_0
      (if (Variables|Default|GetIsAlive)
        (if (<= (Variables|Default|Getm_CurrentHealth) 1.0)
          (CallFunction|DestroyEnemy))))
    (:then_1
      (Utilities|WidgetUpdate))))

(event EventTick
  (params (DeltaSeconds :type Float%20%28single-precision%29))
  (bind _returnvalue (Transformation|GetActorLocation))
  ;[1 1 1] New Dash
  (CallFunction|CalculateVelocity)
  (if (Variables|Default|GetIsAlive)
    (bind _outhit (Collision|SphereTraceByChannel _returnvalue (+ _returnvalue (* (Transformation|GetActorForwardVector) (Variables|Default|GetRange))) 1e+02 "TraceTypeQuery1" false 0 "None"))
    (Utilities|Casting|CastToHMC_Coscoroba (.HitActor (Collision|BreakHitResult _outhit))
      (:then
        (if (Variables|Default|GetAscendTimeLineDone)
          (bind _sppedramp (Timeline|SpeedRamup PlayFromStart)
            (:Update
              (Variables|Default|Setm_Speed (Math|Float|Lerp (Variables|Default|Getm_Speed) (* (Variables|Default|GetinitialSpeed) (Variables|Enemy|GetDashMultiplier)) _sppedramp))
              (Variables|Default|SetAscendTimeLineDone false))
            (:Finished
              (Variables|Default|SetAscendTimeLineDone true)))
          (else
            (Timeline|SpeedRamup Play))))
      (:CastFailed
        (if (> (Variables|Default|Getm_Speed) (Variables|Default|GetinitialSpeed))
          (if (Variables|Default|GetAscendTimeLineDone)
            (if (Variables|Default|GetDescendTimeLineDone)
              (bind _sppedramp_2 (Timeline|SpeedRamDown PlayFromStart)
                (:Update
                  (Variables|Default|Setm_Speed (Math|Float|Lerp (Variables|Default|Getm_Speed) (Variables|Default|GetinitialSpeed) _sppedramp_2))
                  (Variables|Default|SetDescendTimeLineDone false))
                (:Finished
                  (Variables|Default|SetDescendTimeLineDone true)))
              (else
                (Timeline|SpeedRamDown Play)))))))
    (else
      (Utilities|FlowControl|Sequence
        (:then_0
          (Utilities|FlowControl|DoOnce false
            (:Completed
              (Variables|Default|SetFakeVelocity_0 (Math|Vector|MakeVector (* (.x (Variables|Default|GetFakeVelocity_0)) (Variables|Default|Getm_Speed)) (* (.y (Variables|Default|GetFakeVelocity_0)) (Variables|Default|Getm_Speed)) (.z (Variables|Default|GetFakeVelocity_0)))))))
        (:then_1
          (Physics|AddForce (Variables|Default|GetCoreCollider) (Variables|Default|GetFakeVelocity_0) "None" false)
          (Transformation|AddRelativeRotation (Variables|Default|GetMainMesh) (Math|Rotator|MakeRotator 0.0 (* (Utilities|Time|GetWorldDeltaSeconds) 4.0) 0.0) false false))))))

(fn ConstructionScript)

(fn CheckRangeandAttack
  (if (<= (Math|Vector|VectorLength (- (Transformation|GetActorLocation (Variables|Default|GetPlayerRef)) (Transformation|GetActorLocation))) (Variables|Default|GetRange))
    (Variables|Default|SetAttack true)
    (else
      (Variables|Default|SetAttack false))))

(fn DestroyEnemy
  (CallFunction|Explosion)
  (Variables|Default|SetIsAlive false)
  (Effects|Components|ParticleSystem|SetTemplate (Variables|Default|GetParticleSystem) "/Game/StarterContent/Particles/P_Smoke.P_Smoke")
  (Variables|Default|SetMySplineActor 0)
  (Physics|SetEnableGravity (Variables|Default|GetCoreCollider) true))

(fn Explode
  (CallFunction|Explosion)
  (Actor|DestroyActor))

(fn Explosion
  (bind _returnvalue (Transformation|GetActorLocation))
  (Effects|SpawnEmitteratLocation "/Game/StarterContent/Particles/P_Explosion.P_Explosion" _returnvalue "0, 0, 0" "50.000000,50.000000,50.000000")
  (Audio|PlaySoundatLocation "/Game/StarterContent/Audio/Explosion02.Explosion02" _returnvalue "0, 0, 0" 1.0 1.0 0.0 0 0 0))

(fn CalculateVelocity
  (bind _corecollider (Variables|Default|GetCoreCollider))
  (bind _returnvalue (Transformation|GetWorldLocation _corecollider))
  (Variables|Default|SetFakeVelocity_0 (/ (- _returnvalue (Variables|Default|GetPrevPosition)) (Utilities|Time|GetWorldDeltaSeconds)))
  (Variables|Default|SetPrevPosition _returnvalue))

(fn ITGetLocation
  (return (Transformation|GetWorldLocation (Variables|Default|GetMainMesh))))

(fn ITGetRotation
  (bind _mainmesh (Variables|Default|GetMainMesh))
  (bind _returnvalue (Transformation|GetWorldRotation _mainmesh))
  (bind (_roll _pitch _yaw) (Math|Rotator|BreakRotator _returnvalue))
  (return (Math|Rotator|MakeRotator _roll _pitch (+ _yaw 1.0))))

(fn ITIsAlive
  (return (Variables|Default|GetIsAlive)))