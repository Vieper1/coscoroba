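; LightEnemySpawner_BP is a trigger-driven spawner that creates light enemies when the HMC_Coscoroba actor enters its trigger.
; On overlap it loops over LTSpawnStructs and spawns a LightEnemy_BP at the first point of each entry's spline actor, ignoring collisions.
; It then copies that entry's spline, range, firing, speed and aim settings onto the new enemy.
; Nothing disables the trigger, so each qualifying overlap spawns the whole set again.
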(event OnComponentBeginOverlap(Trigger)
  (params (OverlappedComponent :type Primitive%20Component%20Object%20Reference) (OtherActor :type Actor%20Object%20Reference) (OtherComp :type Primitive%20Component%20Object%20Reference) (OtherBodyIndex :type Integer) (bFromSweep :type Boolean) (SweepResult :type Hit%20Result%20Structure%20%28by%20ref%29))
  (Utilities|Casting|CastToHMC_Coscoroba OtherActor)
  (for _array_element (Variables|Default|GetLT_SpawnStructs)
    (bind _returnvalue (Game|SpawnActorfromClass "/Game/Cosco/Blueprints/Enemy/Light/LightEnemy_BP.LightEnemy_BP_C" (Math|Transform|MakeTransform (Spline|GetLocationatSplinePoint (Variables|/Script/Bofor.SplineActor|GetSpline (.SplineActor (Utilities|Struct|BreakLTSpawn_Struct _array_element))) 0 "World") "0, 0, 0" "1,1,1") "AlwaysSpawn" 0 0 0))
    (Utilities|FlowControl|Sequence
      (:then_0
        (Variables|/Script/Bofor.CoscoBaseCharacter|SetMySplineActor _returnvalue (.SplineActor (Utilities|Struct|BreakLTSpawn_Struct _array_element))))
      (:then_1
        (Variables|/Script/Bofor.CoscoEnemyCharacter|SetRange _returnvalue (.Range (Utilities|Struct|BreakLTSpawn_Struct _array_element))))
      (:then_2
        (Variables|/Game/Cosco/Blueprints/Enemy/Light/LightEnemy_BP.LightEnemy_BP_C|SetShoot%20Delay _returnvalue (.FiringDelay (Utilities|Struct|BreakLTSpawn_Struct _array_element))))
      (:then_3
        (Variables|/Script/Bofor.CoscoBaseCharacter|Setm_Speed _returnvalue (.Speed (Utilities|Struct|BreakLTSpawn_Struct _array_element))))
      (:then_4
        (Variables|/Game/Cosco/Blueprints/Enemy/Light/LightEnemy_BP.LightEnemy_BP_C|SetAimWithRandomOffSet _returnvalue (.AimWithRandomOffset (Utilities|Struct|BreakLTSpawn_Struct _array_element))))
      (:then_5
        (Variables|/Game/Cosco/Blueprints/Enemy/Light/LightEnemy_BP.LightEnemy_BP_C|SetAimOffset _returnvalue (.AimOffSet (Utilities|Struct|BreakLTSpawn_Struct _array_element)))))))

(event EventBeginPlay)

(event Collision|EventActorBeginOverlap
  (params (OtherActor :type Actor%20Object%20Reference)))

(event EventTick
  (params (DeltaSeconds :type Float%20%28single-precision%29)))

(fn ConstructionScript)